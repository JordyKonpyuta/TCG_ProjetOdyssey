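; BP_Card is a card actor in a card game, showing its CardData through a WBP_Card widget and tracking stats and attached energies.
; Widget hover and click events drive looping interpolation timers that raise the card, follow the cursor and snap it onto a free BP_CardSlot found by line trace.
; Clicks also handle PC_CardGame target selection or reveal placed-card buttons.
; Health clamping works, but attack effects, stat setters and death are stubs.
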(event `InitializeCard`
  (params (CardData :type "/Game/Blueprints/Datas/PDA_CardStats Object Reference"))
  (bind _carddata (`self.CardData`))
  (set `self.CardData` CardData)
  (bind _aswbp_card (cast `/Game/Blueprints/Widgets/InGame/WBP_Card` (`WidgetComponent.GetWidget` (`self.Widget`))))
  (set `/Game/Blueprints/Widgets/InGame/WBP_Card.CardData` (`self.CardData`) _aswbp_card)
  (`/Game/Blueprints/Widgets/InGame/WBP_Card.InitializeCard` _aswbp_card)
  (`/Game/Blueprints/Widgets/InGame/WBP_Card.ToggleButtonsActivation` _aswbp_card false)
  (set `/Game/Blueprints/Widgets/InGame/WBP_Card.CardReference` self _aswbp_card)
  (set `self.Attack` (`/Game/Blueprints/Datas/PDA_CardStats.Attack` _carddata))
  (set `self.Defense` (`/Game/Blueprints/Datas/PDA_CardStats.Defense` _carddata))
  (set `self.HP` (`/Game/Blueprints/Datas/PDA_CardStats.HP` _carddata)))

(event `self.ReceiveBeginPlay`
  ; Event Begin Play
  (set `self.ControllerRef` (cast `/Game/Blueprints/Core/PC_CardGame` (`GameplayStatics.GetPlayerController` 0) :!pure true)))

(event `self.Widget.OnBeginCursorOver`
  (params (TouchedComponent :type "PrimitiveComponent Object Reference"))
  ; Hover and Unhover card - rise a little the card
  (if (not (`self.IsPlaced`))
    (set `self.Destination` (`SceneComponent.RelativeLocation` (`self.Arrow_Destination`)))
    (bind _returnvalue (`KismetSystemLibrary.K2_SetTimerDelegate` (`|CreateDelegate` :!event `MoveCard`) 0.01 true))
    (set `self.RiseCardTimerHandle` _returnvalue)
    (elif (`self.IsFollowingCursor`)
      (`self.K2_SetActorRelativeLocation` (`SceneComponent.RelativeLocation` (`self.Arrow_Start`))))))

(event `self.Widget.OnEndCursorOver`
  (params (TouchedComponent :type "PrimitiveComponent Object Reference"))
  ; Hover and Unhover card - rise a little the card
  (if (not (`self.IsPlaced`))
    (set `self.Destination` (`SceneComponent.RelativeLocation` (`self.Arrow_Start`)))
    (bind _returnvalue (`KismetSystemLibrary.K2_SetTimerDelegate` (`|CreateDelegate` :!event `MoveCard`) 0.01 true))
    (set `self.RiseCardTimerHandle` _returnvalue)
    (elif (`self.IsFollowingCursor`)
      (`self.K2_SetActorRelativeLocation` (`SceneComponent.RelativeLocation` (`self.Arrow_Start`))))))

(event `MoveCard`
  (bind _staticmesh (`self.StaticMesh`))
  ; Function to call when Hover/Unhover card
  (`SceneComponent.K2_SetRelativeLocation` _staticmesh (`KismetMathLibrary.VInterpTo` (`SceneComponent.RelativeLocation` _staticmesh) (`self.Destination`) (`GameplayStatics.GetWorldDeltaSeconds`) 3.0) false false)
  (if (== (`SceneComponent.RelativeLocation` _staticmesh) (`self.Destination`) :`ErrorTolerance` 50.0)
    (`KismetSystemLibrary.K2_ClearAndInvalidateTimerHandle` (`self.RiseCardTimerHandle`))))

(event `self.Widget.OnClicked`
  (params (TouchedComponent :type "PrimitiveComponent Object Reference") (ButtonPressed :type "Key Structure"))
  (bind _controllerref (`self.ControllerRef`))
  (bind _selectedcards (`/Game/Blueprints/Core/PC_CardGame.SelectedCards` _controllerref))
  (bind _selectedcards_2 (`/Game/Blueprints/Core/PC_CardGame.SelectedCards` (`self.ControllerRef`)))
  ; Click on the card
  (`KismetSystemLibrary.K2_ClearAndInvalidateTimerHandle` (`self.RiseCardTimerHandle`))
  (if (`/Game/Blueprints/Core/PC_CardGame.IsSelectionMode` (`self.ControllerRef`))
    (`/Game/Blueprints/Widgets/InGame/WBP_Card.ToggleButtonsActivation` (cast `/Game/Blueprints/Widgets/InGame/WBP_Card` (`WidgetComponent.GetWidget` (`self.Widget`)) :!pure true) false)
    (if (`KismetArrayLibrary.Array_Contains` _selectedcards self)
      (`KismetArrayLibrary.Array_RemoveItem` _selectedcards self)
      (elif (== (`.NumberOfTargets_28_48B0234F465B0320CAA651B7085942FE` (break `/Game/Blueprints/Datas/S_CardAttacks` (`/Game/Blueprints/Core/PC_CardGame.AttackToUse` _controllerref))) (`/Game/Blueprints/Core/PC_CardGame.NumberOfCardsSelected` (`self.ControllerRef`)))
        (`KismetArrayLibrary.Array_Remove` _selectedcards_2 (`KismetArrayLibrary.Array_LastIndex` _selectedcards_2))
        (`KismetArrayLibrary.Array_AddUnique` _selectedcards_2 self)
        (else
          (`KismetArrayLibrary.Array_AddUnique` _selectedcards_2 self))))
    (elif (not (`self.IsPlaced`))
      (`/Game/Blueprints/Widgets/InGame/WBP_Card.ToggleButtonsActivation` (cast `/Game/Blueprints/Widgets/InGame/WBP_Card` (`WidgetComponent.GetWidget` (`self.Widget`)) :!pure true) false)
      (if (not (`self.IsFollowingCursor`))
        (bind _returnvalue (`KismetSystemLibrary.K2_SetTimerDelegate` (`|CreateDelegate` :!event `SetToMousePosition`) 0.01 true))
        (set `self.CursorTimerHandle` _returnvalue)
        (elif (`self.CanBePlaced`)
          (set `self.IsPlaced` true)
          (set `self.IsFollowingCursor` false)
          (`KismetSystemLibrary.K2_ClearAndInvalidateTimerHandle` (`self.CursorTimerHandle`))
          (bind _returnvalue_2 (`KismetSystemLibrary.K2_SetTimerDelegate` (`|CreateDelegate` :!event `PlaceCardOnSlot`) 0.01 true))
          (set `self.PlaceCardTimerHandle` _returnvalue_2)
          (`KismetArrayLibrary.Array_Add` (`/Game/Blueprints/Core/PC_CardGame.AllPlayerCards` (`self.ControllerRef`)) self)
          (else
            (set `self.IsFollowingCursor` false)
            (`KismetSystemLibrary.K2_ClearAndInvalidateTimerHandle` (`self.CursorTimerHandle`)))))
      (else
        (`/Game/Blueprints/Widgets/InGame/WBP_Card.ToggleButtonsActivation` (cast `/Game/Blueprints/Widgets/InGame/WBP_Card` (`WidgetComponent.GetWidget` (`self.Widget`)) :!pure true) true)))))

(event `SetToMousePosition`
  (bind _returnvalue (`self.K2_GetActorLocation`))
  ; Card Follow cursor position
  (set `self.IsFollowingCursor` true)
  (`self.K2_SetActorLocation` (`KismetMathLibrary.VInterpTo` (`self.K2_GetActorLocation`) (`.Location` (`GameplayStatics.BreakHitResult` (`PlayerController.GetHitResultUnderCursorForObjects` (`self.ControllerRef`) (`|MakeArray` "ObjectTypeQuery1" :!type "EObjectTypeQuery Enum") true))) (`GameplayStatics.GetWorldDeltaSeconds`) 15.0))
  (bind _outhit (`KismetSystemLibrary.LineTraceSingle` (+ _returnvalue (0.0 0.0 500.0)) (- _returnvalue (0.0 0.0 300.0)) "TraceTypeQuery1"))
  (bind _asbp_card_slot (cast `/Game/Blueprints/Core/BP_CardSlot` (`.HitActor` (`GameplayStatics.BreakHitResult` _outhit)))
    (:`then`
      (if (and (`|EnumEquality` (`/Game/Blueprints/Core/BP_CardSlot.SlotType` _asbp_card_slot) "NewEnumerator0") (== (`/Game/Blueprints/Core/BP_CardSlot.CardAttached` _asbp_card_slot) null))
        (set `self.SlotToAttach` _asbp_card_slot)
        (set `self.CanBePlaced` true)
        (else
          (set `self.SlotToAttach` null)
          (set `self.CanBePlaced` false))))
    (:`CastFailed`
      (set `self.SlotToAttach` null)
      (set `self.CanBePlaced` false))))

(event `PlaceCardOnSlot`
  (bind _returnvalue (`SceneComponent.K2_GetComponentToWorld` (`/Game/Blueprints/Core/BP_CardSlot.Arrow` (`self.SlotToAttach`))))
  ; Place card on slot
  (`self.K2_SetActorTransform` (`KismetMathLibrary.TInterpTo` (`self.GetTransform`) _returnvalue (`GameplayStatics.GetWorldDeltaSeconds`) 4.0))
  (if (`KismetMathLibrary.NearlyEqual_TransformTransform` (`self.GetTransform`) _returnvalue 10.0 10.0)
    (`KismetSystemLibrary.K2_ClearAndInvalidateTimerHandle` (`self.PlaceCardTimerHandle`))))

(fn `AttachEnergy`
  (params (EnergyToAttach :type "/Game/Blueprints/Datas/E_EnergyTypes Enum (by ref)"))
  (bind _energiesattached (`self.EnergiesAttached`))
  (bind _returnvalue (`KismetArrayLibrary.Array_Length` _energiesattached))
  (`KismetArrayLibrary.Array_Add` _energiesattached EnergyToAttach)
  (if (< _returnvalue 5)
    (for _index (range _returnvalue)
      (bind _output (`|GetArrayItem` (`|MakeArray` (`self.Energy_1`) (`self.Energy_2`) (`self.Energy_3`) (`self.Energy_4`)) _index))
      (`SceneComponent.SetHiddenInGame` _output false false)
      (`PrimitiveComponent.SetMaterial` _output 0 (select `/Game/Blueprints/Datas/E_EnergyTypes` (`|GetArrayItem` (`self.EnergiesAttached`) _index) :`NewEnumerator0` "/Engine/BasicShapes/BasicShapeMaterial.BasicShapeMaterial" :`NewEnumerator1` "/Engine/BasicShapes/BasicShapeMaterial.BasicShapeMaterial" :`NewEnumerator2` "/Engine/BasicShapes/BasicShapeMaterial.BasicShapeMaterial" :`NewEnumerator3` "/Engine/BasicShapes/BasicShapeMaterial.BasicShapeMaterial" :`NewEnumerator4` "/Engine/BasicShapes/BasicShapeMaterial.BasicShapeMaterial" :`NewEnumerator5` "/Engine/BasicShapes/BasicShapeMaterial.BasicShapeMaterial" :!type "MaterialInterface Object Reference")))
    (else
      (`SceneComponent.SetHiddenInGame` (`self.Energy_1`) false false)
      (`SceneComponent.SetHiddenInGame` (`self.Text_5EnergiesOrMore`) false false)
      (`TextRenderComponent.K2_SetText` (`self.Text_5EnergiesOrMore`) (`KismetTextLibrary.Conv_IntToText` _returnvalue)))))

(fn `CardDeath`)

(fn `SetAttack`)

(fn `SetDefense`)

(fn `SetHealth`
  (params (Value :type Integer))
  (bind _returnvalue (+ Value (`self.HP`)))
  (if (> _returnvalue (`/Game/Blueprints/Datas/PDA_CardStats.HP` (`self.CardData`)))
    (set `self.HP` (`/Game/Blueprints/Datas/PDA_CardStats.HP` (`self.CardData`)))
    (`/Game/Blueprints/Widgets/InGame/WBP_Card.UpdateHealth` (cast `/Game/Blueprints/Widgets/InGame/WBP_Card` (`WidgetComponent.GetWidget` (`self.Widget`)) :!pure true))
    (elif (< _returnvalue 0)
      (set `self.HP` 0)
      (`/Game/Blueprints/Widgets/InGame/WBP_Card.UpdateHealth` (cast `/Game/Blueprints/Widgets/InGame/WBP_Card` (`WidgetComponent.GetWidget` (`self.Widget`)) :!pure true))
      (`self.CardDeath`)
      (else
        (set `self.HP` (+ (`self.HP`) (`local.Value`)))
        (`/Game/Blueprints/Widgets/InGame/WBP_Card.UpdateHealth` (cast `/Game/Blueprints/Widgets/InGame/WBP_Card` (`WidgetComponent.GetWidget` (`self.Widget`)) :!pure true))))))

(fn `UseAttack`
  (params (AttackToUse :type "/Game/Blueprints/Datas/S_CardAttacks Structure"))
  (bind (_name _description _type _energysneeded _effects _effectquantity _debuff _issacrifice_ _isdiscard_ _target) (break `/Game/Blueprints/Datas/S_CardAttacks` AttackToUse))
  (`|ExecutionSequence`
    (:`then_0`
      (switch `/Game/Blueprints/Datas/E_Target` _target
        (:`NewEnumerator3`
          (for _ (`/Game/Blueprints/Core/PC_CardGame.SelectedCards` (`self.ControllerRef`))
            _))
        (:`NewEnumerator5`
          (for _ (`/Game/Blueprints/Core/PC_CardGame.AllPlayerCards` (`self.ControllerRef`))
            _))))
    (:`then_1`
      (switch `/Game/Blueprints/Datas/E_AttackTypes` _type
        (:`NewEnumerator0`
          (set `self.CanBeSelected` false))
        (:`NewEnumerator1`
          (`Widget.SetVisibility` (`/Game/Blueprints/Widgets/InGame/WBP_Attacks.Button_Attack` (cast `/Game/Blueprints/Widgets/InGame/WBP_Attacks` (`PanelWidget.GetChildAt` (`/Game/Blueprints/Widgets/InGame/WBP_Card.VB_Attacks` (cast `/Game/Blueprints/Widgets/InGame/WBP_Card` (`WidgetComponent.GetWidget` (`self.Widget`)) :!pure true)) (`KismetArrayLibrary.Array_Find` (`/Game/Blueprints/Datas/PDA_CardStats.Attacks` (`self.CardData`)) AttackToUse)) :!pure true)) "SelfHitTestInvisible"))))))

(fn `UserConstructionScript`)