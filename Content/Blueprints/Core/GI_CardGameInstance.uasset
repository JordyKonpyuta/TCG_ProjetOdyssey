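; Card game's GameInstance that owns the global save and generates random bosses.
; Init loads the "Global" save or creates one with Mochiyo as the default character.
; GenerateRandomBoss stores a random boss, difficulty-scaled feature count and conditional debuff in that difficulty's save slot entry, then saves.
; Feature picking retries on duplicates, though the check re-rolls instead of testing the picked feature.
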(event `self.ReceiveInit`
  (bind _returnvalue (`GameplayStatics.DoesSaveGameExist` "Global"))
  (if _returnvalue
    (bind _returnvalue_2 (`GameplayStatics.LoadGameFromSlot` "Global"))
    (bind _asbp_card_game_save_system (cast `/Game/Blueprints/Core/BP_CardGameSaveSystem` _returnvalue_2))
    (set `self.SaveGameSystem` _asbp_card_game_save_system)
    (else
      (bind _returnvalue_3 (`GameplayStatics.CreateSaveGameObject` "/Game/Blueprints/Core/BP_CardGameSaveSystem.BP_CardGameSaveSystem_C"))
      (bind _output_get (set `self.SaveGameSystem` _returnvalue_3))
      (bind _returnvalue_4 (`|GetDataTableRow` "/Game/Blueprints/Datas/SaveSystem/DT_Characters.DT_Characters" "Mochiyo")
        (:`then`
          (set `/Game/Blueprints/Core/BP_CardGameSaveSystem.SelectedCharacter` _returnvalue_4 _output_get)
          (`GameplayStatics.SaveGameToSlot` _output_get "Global"))))))

(fn `GenerateRandomBoss`
  (locals (AvailableFeatures :type "Array of /Game/Blueprints/Datas/Boss/E_BossFeatures Enum") (PickedFeatures :type "Array of /Game/Blueprints/Datas/Boss/E_BossFeatures Enum") (NumberOfFeaturesToPick :type "Array of Integer") (AvailableDebuffs :type "Array of /Game/Blueprints/Datas/Cards/Characters/E_Debuffs Enum") (PickedFeature :type "/Game/Blueprints/Datas/Boss/E_BossFeatures Enum" :default "NewEnumerator0"))
  (bind _pickedfeatures (`local.PickedFeatures`))
  (bind _outitem (`KismetArrayLibrary.Array_Random` (`local.AvailableFeatures`)))
  (bind _returnvalue (select `/Game/Blueprints/Datas/Boss/E_Difficulty` (`self.Difficulty`) :`NewEnumerator1` 1 :`NewEnumerator2` 2 :`NewEnumerator3` 3 :`NewEnumerator4` 4))
  (bind _output (`|GetArrayItem` (`/Game/Blueprints/Core/BP_CardGameSaveSystem.SavedBoss` (`self.SaveGameSystem`)) _returnvalue))
  (bind _returnvalue_2 (`|GetDataTableRow` "/Game/Blueprints/Datas/Boss/DT_Boss.DT_Boss" (`KismetArrayLibrary.Array_Random` (`|MakeArray` "Dragon" "Kraken" "Angel" :!type "Name")))
    (:`then`
      (setmembers `/Game/Blueprints/Datas/SaveSystem/S_SavedBoss` :`StructRef` _output :`Boss` _returnvalue_2)
      (for _ (range (`|GetArrayItem` (`local.NumberOfFeaturesToPick`) _returnvalue))
        (set `local.PickedFeature` _outitem :!label _label)
        (if (not (`KismetArrayLibrary.Array_Contains` (`local.PickedFeatures`) _outitem))
          (`KismetArrayLibrary.Array_AddUnique` (`local.PickedFeatures`) (`local.PickedFeature`))
          (else
            (goto _label))))
      (setmembers `/Game/Blueprints/Datas/SaveSystem/S_SavedBoss` :`StructRef` _output :`Features` _pickedfeatures)
      (if (or (`KismetArrayLibrary.Array_Contains` _pickedfeatures "NewEnumerator3") (`KismetArrayLibrary.Array_Contains` _pickedfeatures "NewEnumerator2") (`KismetArrayLibrary.Array_Contains` _pickedfeatures "NewEnumerator1"))
        (setmembers `/Game/Blueprints/Datas/SaveSystem/S_SavedBoss` :`StructRef` _output :`Debuff` (`KismetArrayLibrary.Array_Random` (`local.AvailableDebuffs`)))
        (else
          (setmembers `/Game/Blueprints/Datas/SaveSystem/S_SavedBoss` :`StructRef` _output :`Debuff` "NewEnumerator6")))
      (`GameplayStatics.SaveGameToSlot` (`self.SaveGameSystem`) "Global"))))