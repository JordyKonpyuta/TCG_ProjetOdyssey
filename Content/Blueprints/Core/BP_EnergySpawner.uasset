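; BP_EnergySpawner is an actor that spawns a BP_Energy at its own transform on BeginPlay.
; It gives the new energy a reference back to itself and a type picked from its EnergiesToSpawn array.
; The pick uses a random stream created with a fixed seed, so it repeats for a given array length.
; The random range's upper bound is the array length, one past the last valid index.
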(event `self.ReceiveBeginPlay`
  (bind _energiestospawn (`self.EnergiesToSpawn`))
  (bind _returnvalue (`KismetArrayLibrary.Array_Length` _energiestospawn))
  (bind _returnvalue_2 (`|SpawnActorFromClass` "/Game/Blueprints/Core/BP_Energy.BP_Energy_C" (`self.GetTransform`) "Undefined" "MultiplyWithRoot" null null))
  (set `/Game/Blueprints/Core/BP_Energy.EnergySpawner` self _returnvalue_2)
  (set `/Game/Blueprints/Core/BP_Energy.EnergyType` (`|GetArrayItem` _energiestospawn (select `bool` (> _returnvalue 0) :`true` (`KismetMathLibrary.RandomIntegerInRangeFromStream` (`KismetMathLibrary.MakeRandomStream` 0) 0 _returnvalue))) _returnvalue_2))

(fn `UserConstructionScript`)