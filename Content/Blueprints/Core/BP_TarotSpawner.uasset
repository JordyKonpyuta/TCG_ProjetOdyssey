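; Spawner actor that offers a random set of tarot cards during the card game, with fewer cards when the boss has a specific feature.
; It registers itself on PC_CardGame, and its turn check combines a random-interval modulo with a random pick from a chance array.
; Spawning hides the HUD, switches music, fills a WBP_TarotSpawn widget with unique BP_CardData objects via retry-on-duplicate picks, and moves the camera.
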(event `self.ReceiveBeginPlay`
  (bind _aspc_card_game (cast `/Game/Blueprints/Core/PC_CardGame` (`GameplayStatics.GetPlayerController` 0) :!pure true))
  (`KismetSystemLibrary.Delay` 0.5)
  (set `/Game/Blueprints/Core/PC_CardGame.TarotSpawnerRef` self _aspc_card_game)
  (bind _output_get (set `self.PlayerControllerRef` _aspc_card_game))
  (set `self.NumberOfCardsToSpawn` (select `bool` (`KismetArrayLibrary.Array_Contains` (`/Game/Blueprints/Core/Ennemies/BP_Ennemy_Master.Features` (`/Game/Blueprints/Core/PC_CardGame.BossRef` _output_get)) "NewEnumerator9") :`false` 5 :`true` 3)))

(event `SpawnCards`
  (bind _playercontrollerref (`self.PlayerControllerRef`))
  (`Widget.SetVisibility` (`/Game/Blueprints/Core/PC_CardGame.HUD_Ref` _playercontrollerref) "Collapsed")
  (`KismetSystemLibrary.Delay` 1.0)
  (`/Game/Blueprints/Core/BP_CameraPlayer.ChangeMusic` (`/Game/Blueprints/Core/PC_CardGame.CameraRef` _playercontrollerref) "/Game/Assets/Sounds/Musics/Cues/A_Tarot_Cue.A_Tarot_Cue")
  (`KismetArrayLibrary.Array_Clear` (`self.SpawnedTarotCards`))
  (bind _returnvalue (`|CreateWidget` "/Game/Blueprints/Widgets/InGame/WBP_TarotSpawn.WBP_TarotSpawn_C"))
  (bind _output_get (set `/Game/Blueprints/Core/PC_CardGame.TarotUI_Ref` _returnvalue (`self.PlayerControllerRef`)))
  (`UserWidget.AddToViewport` _output_get 0)
  (for _index (range (+ (`self.NumberOfCardsToSpawn`) 1))
    (while (not (`KismetArrayLibrary.Array_IsValidIndex` (`self.SpawnedTarotCards`) _index))
      (set `self.TarotPicked` (`KismetArrayLibrary.Array_Random` (`self.AvailableTarotDatas`)))
      (if (not (`KismetArrayLibrary.Array_Contains` (`self.SpawnedTarotCards`) (`self.TarotPicked`)))
        (bind _returnvalue_2 (`|GenericCreateObject` "/Game/Blueprints/Core/Cards/BP_CardData.BP_CardData_C" "NewEnumerator5"))
        (set `/Game/Blueprints/Core/Cards/BP_CardData.TarotData` (`self.TarotPicked`) _returnvalue_2)
        (`/Game/Blueprints/Widgets/InGame/WBP_TarotSpawn.SpawnTarotCards` _returnvalue _returnvalue_2)
        (`KismetArrayLibrary.Array_AddUnique` (`self.SpawnedTarotCards`) (`self.TarotPicked`)))))
  (`/Game/Blueprints/Core/PC_CardGame.CameraMovement` (`self.PlayerControllerRef`) (`SceneComponent.K2_GetComponentToWorld` (`self.Arrow_CameraPosition`))))

(fn `ShouldSpawnTarotThisTurn`
  (locals (ChancesToPickTarot :type "Array of Boolean"))
  (if (== (mod (`/Game/Blueprints/Core/PC_CardGame.Turn` (`self.PlayerControllerRef`)) (`KismetMathLibrary.RandomIntegerInRange` 3 5)) 0)
    (if (`KismetArrayLibrary.Array_Random` (`local.ChancesToPickTarot`))
      (`self.SpawnCards`)
      (`KismetSystemLibrary.PrintString` "Should Spawn Tarot" true true (struct :`R` 0.27195 :`G` 0.58844 :`B` 1.0 :`A` 1.0)))))

(fn `UserConstructionScript`)