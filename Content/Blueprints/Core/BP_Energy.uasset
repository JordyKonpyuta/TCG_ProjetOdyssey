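; BP_Energy is a clickable energy token for a card game that the player picks up and drops onto cards, with a timeline scaling its mesh in on spawn.
; Clicking with no energy held registers it on PC_CardGame and starts cursor following through looping timers and VInterpTo.
; Clicking while holding traces vertically: hitting a BP_Card attaches the EnergyType and destroys the token, otherwise it glides back to its spawner.
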(event `self.ReceiveBeginPlay`
  (bind _staticmesh (`self.StaticMesh`))
  (bind (_returnvalue_location _returnvalue_rotation) (`KismetMathLibrary.BreakTransform` (`SceneComponent.K2_GetComponentToWorld` _staticmesh)))
  ; Event Begin Play
  (set `self.PlayerControllerRef` (cast `/Game/Blueprints/Core/PC_CardGame` (`GameplayStatics.GetPlayerController` 0) :!pure true))
  (bind (_direction _scale) (`Timeline|T_SpawnEnergy`)
    (:`Update`
      (`SceneComponent.K2_SetWorldTransform` _staticmesh (`KismetMathLibrary.MakeTransform` _returnvalue_location _returnvalue_rotation (`KismetMathLibrary.MakeVector` _scale _scale _scale)) false false))))

(event `self.StaticMesh.OnClicked`
  (params (TouchedComponent :type "PrimitiveComponent Object Reference") (ButtonPressed :type "Key Structure"))
  (bind _returnvalue (`self.K2_GetActorLocation`))
  ; Click on energy
  (if (== (`/Game/Blueprints/Core/PC_CardGame.EnergyAttached` (`self.PlayerControllerRef`)) null)
    (set `/Game/Blueprints/Core/PC_CardGame.EnergyAttached` self (`self.PlayerControllerRef`))
    (bind _returnvalue_2 (`KismetSystemLibrary.K2_SetTimerDelegate` (`|CreateDelegate` :!event `MoveToCursor`) 0.01 true))
    (set `self.CursorTimerHandle` _returnvalue_2)
    (else
      (bind _outhit (`KismetSystemLibrary.LineTraceSingle` (+ _returnvalue (0.0 0.0 300.0)) (- _returnvalue (0.0 0.0 500.0)) "TraceTypeQuery1"))
      (bind _asbp_card (cast `/Game/Blueprints/Core/BP_Card` (`.HitActor` (`GameplayStatics.BreakHitResult` _outhit)))
        (:`then`
          (`/Game/Blueprints/Core/BP_Card.AttachEnergy` _asbp_card (`self.EnergyType`))
          (`KismetSystemLibrary.K2_ClearAndInvalidateTimerHandle` (`self.CursorTimerHandle`))
          (set `/Game/Blueprints/Core/PC_CardGame.EnergyAttached` null (`self.PlayerControllerRef`))
          (`self.K2_DestroyActor`))
        (:`CastFailed`
          (`KismetSystemLibrary.K2_ClearAndInvalidateTimerHandle` (`self.CursorTimerHandle`))
          (bind _returnvalue_3 (`KismetSystemLibrary.K2_SetTimerDelegate` (`|CreateDelegate` :!event `MoveToSpawner`) 0.01 true))
          (set `self.SpawnerTimerHandle` _returnvalue_3)
          (set `/Game/Blueprints/Core/PC_CardGame.EnergyAttached` null (`self.PlayerControllerRef`)))))))

(event `MoveToCursor`
  ; Follow cursor position
  (`self.K2_SetActorLocation` (`KismetMathLibrary.VInterpTo` (`self.K2_GetActorLocation`) (`.Location` (`GameplayStatics.BreakHitResult` (`PlayerController.GetHitResultUnderCursorForObjects` (`self.PlayerControllerRef`) (`|MakeArray` "ObjectTypeQuery1" :!type "EObjectTypeQuery Enum") true))) (`GameplayStatics.GetWorldDeltaSeconds`) 15.0)))

(event `MoveToSpawner`
  (bind _returnvalue (`self.K2_GetActorLocation`))
  (bind _returnvalue_2 (`self.K2_GetActorLocation` (`self.EnergySpawner`)))
  ; Go Back to spawner
  (`self.K2_SetActorLocation` (`KismetMathLibrary.VInterpTo` _returnvalue _returnvalue_2 (`GameplayStatics.GetWorldDeltaSeconds`) 15.0))
  (if (== _returnvalue _returnvalue_2 :`ErrorTolerance` 20.0)
    (`KismetSystemLibrary.K2_ClearAndInvalidateTimerHandle` (`self.SpawnerTimerHandle`))))

(fn `UserConstructionScript`)