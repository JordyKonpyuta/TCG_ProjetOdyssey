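; Boss minion enemy that takes its attack in a turn-based card battle, then triggers the next minion or returns the turn to the player.
; A looping timer interpolates it toward a random card, then it deals damage with critical and table-type bonuses, plays a montage and snaps back to its slot.
; A madness status randomly selects a card or fellow minion as target.
; On death, it updates its boss slot and passes remaining damage to the boss.
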(event `self.ReceiveBeginPlay`
  ; Begin Play
  (set `self.IsBoss` false)
  (`parent.ReceiveBeginPlay`)
  (add `self.EnnemyDeath` (`|CreateDelegate` :!event `MinionDeath`)))

(event `MinionAttack`
  ; Minion Attack
  (set `self.Card to Target` null)
  (set `self.Minion to Target` null)
  (if (`|EnumInequality` (`self.Status`) "NewEnumerator4")
    (bind _canact (`self.VerifyStatus`))
    (if _canact
      (bind _cardtotarget (`self.ChooseRandomTarget` true))
      (set `self.Card to Target` _cardtotarget)
      (bind _returnvalue (`KismetSystemLibrary.K2_SetTimerDelegate` (`|CreateDelegate` :!event `MoveToTarget`) 0.05 true))
      (set `self.MoveTimerHandle` _returnvalue))
    (else
      (`self.MinionMadnessAction`))))

(event `MinionDeath`
  (bind _bossref (`self.BossRef`))
  (bind _output (`|GetArrayItem` (`/Game/Blueprints/Core/Ennemies/BP_Ennemy_Master.MinionsSlots` (`self.BossRef`)) (`self.Index`)))
  ; Minion Death
  (set `/Game/Blueprints/Core/Cards/BP_CardSlot.IsEmpty` false _output)
  (set `/Game/Blueprints/Core/Cards/BP_CardSlot.MinionRef` null _output)
  (`self.SetHealth` _bossref (- (`self.DamageRemains`) (`/Game/Blueprints/Core/Ennemies/BP_Ennemy_Master.Defense` _bossref)))
  (`self.K2_DestroyActor`))

(event `MoveToTarget`
  (bind _returnvalue (`self.K2_GetActorLocation` (select `bool` (`KismetSystemLibrary.IsValid` (`self.Card to Target`)) :`false` (`self.Minion to Target`) :`true` (`/Game/Blueprints/Core/Cards/BP_Card.SlotToAttach` (`self.Card to Target`)) :!type "Actor Object Reference")))
  ; Move to Target
  (set `self.IsWalking` true)
  (`self.K2_SetActorLocation` (`KismetMathLibrary.VInterpTo` (`self.K2_GetActorLocation`) _returnvalue (`GameplayStatics.GetWorldDeltaSeconds`) 5.0))
  (if (== (`self.K2_GetActorLocation`) _returnvalue :`ErrorTolerance` 100.0)
    (`KismetSystemLibrary.K2_ClearAndInvalidateTimerHandle` (`self.MoveTimerHandle`))
    (set `self.IsWalking` false)
    (`self.AttackTarget` (`self.Card to Target`) (`self.Minion to Target`))))

(event `AttackTarget`
  (params (CardToTarget :type "/Game/Blueprints/Core/Cards/BP_Card_Character Object Reference") (MinionToTarget :type "/Game/Blueprints/Core/Ennemies/Minions/BP_Ennemy_Minion Object Reference"))
  (bind _iscriticalhit (`self.CheckCriticalHit`))
  (bind _returnvalue (+ (`self.Index`) 1))
  (bind _minionsslots (`/Game/Blueprints/Core/Ennemies/BP_Ennemy_Master.MinionsSlots` (`self.BossRef`)))
  (bind _minionref (`/Game/Blueprints/Core/Cards/BP_CardSlot.MinionRef` (`|GetArrayItem` _minionsslots _returnvalue)))
  ; Attack Target
  (`/Engine/EditorBlueprintResources/StandardMacros.IsValid` CardToTarget
    (:`Is Valid`
      (`/Game/Blueprints/Core/Cards/BP_Card_Character.SetHealth` CardToTarget (`KismetMathLibrary.FTrunc` (* (* (- (`/Game/Blueprints/Core/Cards/BP_Card_Character.Defense` CardToTarget) (`self.Attack`)) (select `bool` (`self.CheckTableType` CardToTarget) :`false` 1.0 :`true` 1.2 :!type "Float (single-precision)")) (select `bool` (`self.CheckCriticalHit`) :`false` 1.0 :`true` 1.2))) self null))
    (:`Is Not Valid`
      (`self.SetHealth` MinionToTarget (`KismetMathLibrary.FTrunc` (* (- (`/Game/Blueprints/Core/Ennemies/BP_Ennemy_Master.Defense` MinionToTarget) (`self.Attack`)) (select `bool` _iscriticalhit :`false` 1.0 :`true` 1.2 :!type "Float (single-precision)"))))))
  (`|PlayMontage` (`self.SkeletalMesh`) (select `bool` _iscriticalhit :`false` (`self.Anim_Attack_Normal`) :`true` (`self.Anim_Attack_Big`))
    (:`OnCompleted`
      (`self.K2_SetActorLocation` (`SceneComponent.K2_GetComponentLocation` (`/Game/Blueprints/Core/Cards/BP_CardSlot.Arrow` (`|GetArrayItem` (`/Game/Blueprints/Core/Ennemies/BP_Ennemy_Master.MinionsSlots` (`self.BossRef`)) (`self.Index`)))))
      (`KismetSystemLibrary.Delay` 1.0)
      (if (`KismetArrayLibrary.Array_IsValidIndex` _minionsslots _returnvalue)
        (`/Engine/EditorBlueprintResources/StandardMacros.IsValid` _minionref
          (:`Is Valid`
            (`self.MinionAttack` _minionref))
          (:`Is Not Valid`
            (`/Game/Blueprints/Core/PC_CardGame.StartPlayerTurn` (`self.PlayerControllerRef`) :!label _label)))
        (else
          (goto _label))))
    (:`OnInterrupted`
      (`KismetSystemLibrary.PrintString` "Animation Failed"))))

(fn `MinionMadnessAction`
  (if (`KismetMathLibrary.RandomBool`)
    (bind _cardtotarget (`self.ChooseRandomTarget` true))
    (set `self.Card to Target` _cardtotarget)
    (`KismetSystemLibrary.K2_SetTimerDelegate` _)
    (else
      (bind (_cardtotarget_2 _miniontotarget) (`self.ChooseRandomTarget` false))
      (set `self.Minion to Target` _miniontotarget))))

(fn `UserConstructionScript`
  (`parent.UserConstructionScript`))