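; Blue minion enemy Blueprint, a child variant that relies on its parent class for its logic.
; On BeginPlay it runs the parent logic, then initializes its WBP_MinionHealthBar widget with its current and max HP and the blue normal and focused bar textures.
; Tick and overlap events are disabled stubs, and the construction script only calls the parent.
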(event `self.ReceiveBeginPlay`
  (`parent.ReceiveBeginPlay`)
  (`/Game/Blueprints/Widgets/InGame/WBP_MinionHealthBar.InitializeBar` (cast `/Game/Blueprints/Widgets/InGame/WBP_MinionHealthBar` (`WidgetComponent.GetWidget` (`self.Widget_HealthBar`)) :!pure true) (`self.HP`) (`self.MaxHP`) "/Game/Assets/Textures/UI/Bars/Ennemies/Focused/T_HealthBar_Blue_F.T_HealthBar_Blue_F" "/Game/Assets/Textures/UI/Bars/Ennemies/Normal/T_HealthBar_Blue.T_HealthBar_Blue"))

(fn `UserConstructionScript`
  (`parent.UserConstructionScript`))