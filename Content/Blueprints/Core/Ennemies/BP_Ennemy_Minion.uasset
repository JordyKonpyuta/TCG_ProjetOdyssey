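; Minion enemy for a turn-based card battle, a non-boss enemy child that attacks during the enemy turn.
; MinionAttack hits a random player attack card if one specific Status value passes VerifyStatus; other statuses trigger MinionMadnessAction, which randomly hits a card or boss minion.
; Damage sets health to Defense minus Attack, using separate Random calls for target and Defense.
; After one second it chains to the next slot's minion or starts the player turn.
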(event `self.ReceiveBeginPlay`
  (set `self.IsBoss` false)
  (`parent.ReceiveBeginPlay`))

(event `MinionAttack`
  (bind _returnvalue (+ (`self.Index`) 1))
  (bind _minionsslots (`/Game/Blueprints/Core/Ennemies/BP_Ennemy_Master.MinionsSlots` (`self.BossRef`)))
  (bind _outitem (`KismetArrayLibrary.Array_Random` (`/Game/Blueprints/Core/PC_CardGame.PlayerAttackCards` (`self.PlayerControllerRef`))))
  (`|ExecutionSequence`
    (:`then_0`
      (if (`|EnumEquality` (`self.Status`) "NewEnumerator4")
        (bind _canact (`self.VerifyStatus`))
        (if _canact
          (`/Game/Blueprints/Core/Cards/BP_Card_Character.SetHealth` _outitem (- (`/Game/Blueprints/Core/Cards/BP_Card_Character.Defense` _outitem) (`self.Attack`)) null null))
        (else
          (`self.MinionMadnessAction`))))
    (:`then_1`
      (`KismetSystemLibrary.Delay` 1.0)
      (if (`KismetArrayLibrary.Array_IsValidIndex` _minionsslots _returnvalue)
        (`self.MinionAttack` (`/Game/Blueprints/Core/Cards/BP_CardSlot.MinionRef` (`|GetArrayItem` _minionsslots _returnvalue)))
        (else
          (`/Game/Blueprints/Core/PC_CardGame.StartPlayerTurn` (`self.PlayerControllerRef`)))))))

(fn `MinionMadnessAction`
  (bind _outitem (`KismetArrayLibrary.Array_Random` (`/Game/Blueprints/Core/PC_CardGame.PlayerAttackCards` (`self.PlayerControllerRef`))))
  (bind _minionref (`/Game/Blueprints/Core/Cards/BP_CardSlot.MinionRef` (`KismetArrayLibrary.Array_Random` (`/Game/Blueprints/Core/Ennemies/BP_Ennemy_Master.MinionsSlots` (`self.BossRef`)))))
  (if (`KismetMathLibrary.RandomBool`)
    (`/Game/Blueprints/Core/Cards/BP_Card_Character.SetHealth` _outitem (- (`/Game/Blueprints/Core/Cards/BP_Card_Character.Defense` _outitem) (`self.Attack`)) null null)
    (else
      (`self.SetHealth` _minionref (- (`/Game/Blueprints/Core/Ennemies/BP_Ennemy_Master.Defense` _minionref) (`self.Attack`))))))

(fn `UserConstructionScript`
  (`parent.UserConstructionScript`))