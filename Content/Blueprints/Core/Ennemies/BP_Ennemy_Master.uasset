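; Base enemy for the card game, shared by bosses and minions, with DT_Boss stats scaled down for minions.
; Bosses spawn difficulty-based minion slots, and dead minions pass leftover damage to their boss.
; BossAttack randomly picks summons, heavy or base attacks, using status checks and shuffled bool arrays as odds on some paths.
; Attacks can inflict statuses on player cards, or on the boss's own minions under Madness.
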(event `self.ReceiveBeginPlay`
  ; Begin Play
  (`|ExecutionSequence`
    (:`then_0`
      (bind _returnvalue (`|GetDataTableRow` "/Game/Blueprints/Datas/Boss/DT_Boss.DT_Boss" (`KismetStringLibrary.Conv_StringToName` (`self.Name`)))
        (:`then`
          (bind ((`Type_25_720CE45B40CB627A15D6969D47A172EA` _type) (`HP_7_6FBAA1704A1E252C1802D2B3CA690ED3` _hp) (`Attack_9_31568C9D414FDE5D065BEFA05D4C8E72` _attack) (`Defense_11_1835DDD24D9A6CC462232E93B386880C` _defense)) (break `/Game/Blueprints/Datas/Boss/S_Boss` _returnvalue))
          (set `self.Type` _type)
          (set `self.MaxHP` (select `bool` (`self.IsBoss`) :`false` (* _hp (`self.MinionStatPercentage`)) :`true` _hp))
          (set `self.Attack` (select `bool` (`self.IsBoss`) :`false` (* _attack (`self.MinionStatPercentage`)) :`true` _attack))
          (set `self.Defense` (select `bool` (`self.IsBoss`) :`false` (* _defense (`self.MinionStatPercentage`)) :`true` _defense)))))
    (:`then_1`
      (set `self.PlayerControllerRef` (cast `/Game/Blueprints/Core/PC_CardGame` (`GameplayStatics.GetPlayerController` 0) :!pure true)))
    (:`then_2`
      (if (`self.IsBoss`)
        (`self.InitializeSlots`)
        (set `/Game/Blueprints/Core/PC_CardGame.BossRef` self (`self.PlayerControllerRef`))))))

(event `InitializeSlots`
  ; Initialize Minions Slots
  (for _index (range (+ (select `/Game/Blueprints/Datas/Boss/E_Difficulty` (`/Game/Blueprints/Core/GI_CardGameInstance.Difficulty` (cast `/Game/Blueprints/Core/GI_CardGameInstance` (`GameplayStatics.GetGameInstance`) :!pure true)) :`NewEnumerator0` 2 :`NewEnumerator1` 2 :`NewEnumerator2` 3 :`NewEnumerator3` 4 :`NewEnumerator4` 5) 1))
    (bind _returnvalue (`|SpawnActorFromClass` "/Game/Blueprints/Core/Cards/BP_CardSlot.BP_CardSlot_C" (`SceneComponent.K2_GetComponentToWorld` (`|GetArrayItem` (`|MakeArray` (`self.Arrow_1`) (`self.Arrow_2`) (`self.Arrow_3`) (`self.Arrow_4`) (`self.Arrow_5`) (`self.Arrow_6`)) _index)) "Undefined" "MultiplyWithRoot" null null))
    (set `/Game/Blueprints/Core/Cards/BP_CardSlot.SlotType` "NewEnumerator1" _returnvalue)
    (set `/Game/Blueprints/Core/Cards/BP_CardSlot.IsEmpty` false _returnvalue)
    (`KismetArrayLibrary.Array_Add` (`self.MinionsSlots`) _returnvalue)))

(event `BaseAttack`
  (bind _outitem (`KismetArrayLibrary.Array_Random` (`/Game/Blueprints/Core/PC_CardGame.PlayerAttackCards` (`self.PlayerControllerRef`))))
  (bind _minionref (`/Game/Blueprints/Core/Cards/BP_CardSlot.MinionRef` (`KismetArrayLibrary.Array_Random` (`self.MinionsSlots`))))
  ; Boss Actions
  (if (select `bool` (`|EnumEquality` (`self.Status`) "NewEnumerator4") :`false` true :`true` (`KismetMathLibrary.RandomBool`))
    (`/Game/Blueprints/Core/Cards/BP_Card_Character.SetHealth` _outitem (- (`/Game/Blueprints/Core/Cards/BP_Card_Character.Defense` _outitem) (`self.Attack`)) self null)
    (`self.InflictStatus` _outitem)
    (else
      (`self.SetHealth` _minionref (- (`/Game/Blueprints/Core/Ennemies/BP_Ennemy_Master.Defense` _minionref) (`self.Attack`)))
      (`self.InflictStatus` null _minionref))))

(event `HeavyAttack`
  ; Boss Actions
  (if (select `bool` (`|EnumEquality` (`self.Status`) "NewEnumerator4") :`false` true :`true` (`KismetMathLibrary.RandomBool`))
    (for _array_element (`/Game/Blueprints/Core/PC_CardGame.PlayerAttackCards` (`self.PlayerControllerRef`))
      (`/Game/Blueprints/Core/Cards/BP_Card_Character.SetHealth` _array_element (- (`/Game/Blueprints/Core/Cards/BP_Card_Character.Defense` _array_element) (`self.Attack`)) self null)
      (`self.InflictStatus` _array_element))
    (else
      (for _array_element_2 (`self.MinionsSlots`)
        (bind _minionref (`/Game/Blueprints/Core/Cards/BP_CardSlot.MinionRef` _array_element_2))
        (`self.SetHealth` _minionref (- (`/Game/Blueprints/Core/Ennemies/BP_Ennemy_Master.Defense` _minionref) (`self.Attack`)))
        (`self.InflictStatus` null _minionref)))))

(event `SpawnMinions`
  ; Boss Actions
  (for (_array_element _array_index) (`self.MinionsSlots`)
    (if (`/Game/Blueprints/Core/Cards/BP_CardSlot.IsEmpty` _array_element)
      (bind _returnvalue (`|GetDataTableRow` "/Game/Blueprints/Datas/Boss/DT_Boss.DT_Boss" (`KismetStringLibrary.Conv_StringToName` (`self.Name`)))
        (:`then`
          (bind _returnvalue_2 (`|SpawnActorFromClass` (`.Minions_21_71312B1942620401188169823BD64341` (break `/Game/Blueprints/Datas/Boss/S_Boss` _returnvalue)) (`self.GetTransform` _array_element) "Undefined" "MultiplyWithRoot" null null))
          (bind _asbp_ennemy_minion (cast `/Game/Blueprints/Core/Ennemies/BP_Ennemy_Minion` _returnvalue_2))
          (set `/Game/Blueprints/Core/Ennemies/BP_Ennemy_Minion.Index` _array_index _asbp_ennemy_minion)
          (set `/Game/Blueprints/Core/Ennemies/BP_Ennemy_Minion.BossRef` self _asbp_ennemy_minion)
          (set `/Game/Blueprints/Core/Cards/BP_CardSlot.IsEmpty` false _array_element))))))

(event `StartMinionsSequence`
  ; Start Minion Sequence
  (`KismetSystemLibrary.Delay` 1.0)
  (`/Game/Blueprints/Core/Ennemies/BP_Ennemy_Minion.MinionAttack` (`/Game/Blueprints/Core/Cards/BP_CardSlot.MinionRef` (`|GetArrayItem` (`self.MinionsSlots`)))))

(fn `BossAttack`
  (locals (EmptySlotsAmount :type Integer) (ChancesToDoAction :type "Array of Boolean"))
  (bind _chancestodoaction (`local.ChancesToDoAction`))
  (bind _chancestodoaction_2 (`local.ChancesToDoAction`))
  (bind _chancestodoaction_3 (`local.ChancesToDoAction`))
  (bind _chancestodoaction_4 (`local.ChancesToDoAction`))
  (bind _chancestodoaction_5 (`local.ChancesToDoAction`))
  (bind _chancestodoaction_6 (`local.ChancesToDoAction`))
  (bind _returnvalue (`KismetArrayLibrary.Array_Length` (`self.MinionsSlots`)))
  (bind _turn (`/Game/Blueprints/Core/PC_CardGame.Turn` (`self.PlayerControllerRef`)))
  (bind _turn_2 (`/Game/Blueprints/Core/PC_CardGame.Turn` (`self.PlayerControllerRef`)))
  (if (`|EnumInequality` (`self.Status`) "NewEnumerator6")
    (bind _canact (`self.VerifyStatus`))
    (if _canact
      (for _array_element (`self.MinionsSlots`)
        (if (`/Game/Blueprints/Core/Cards/BP_CardSlot.IsEmpty` _array_element)
          (`/Engine/EditorBlueprintResources/StandardMacros.IncrementInt` (`local.EmptySlotsAmount`))))
      (if (!= (`local.EmptySlotsAmount`) 0)
        (for _ (range 2)
          (`KismetArrayLibrary.Array_Add` (`local.ChancesToDoAction`)))
        (`|ExecutionSequence`
          (:`then_0`
            (if (>= (`local.EmptySlotsAmount`) (/ _returnvalue 2))
              (`KismetArrayLibrary.Array_Remove` _chancestodoaction_6 (`KismetArrayLibrary.Array_LastIndex` _chancestodoaction_6))))
          (:`then_1`
            (if (== _returnvalue (`local.EmptySlotsAmount`))
              (`KismetArrayLibrary.Array_Remove` _chancestodoaction_5 (`KismetArrayLibrary.Array_LastIndex` _chancestodoaction_5))))
          (:`then_2`
            (`KismetArrayLibrary.Array_Shuffle` (`local.ChancesToDoAction`))
            (if (`KismetArrayLibrary.Array_Random` (`local.ChancesToDoAction`))
              (`self.SpawnMinions`)
              (`self.StartMinionsSequence`)
              (return)
              (else
                (`KismetArrayLibrary.Array_Clear` _chancestodoaction)
                (`KismetArrayLibrary.Array_Add` _chancestodoaction true)
                (if (and (>= _turn 5) (< _turn 10)) :!label _label
                  (for _ (range 7)
                    (`KismetArrayLibrary.Array_Add` (`local.ChancesToDoAction`)))
                  (`|ExecutionSequence`
                    (:`then_0`
                      (if (and (>= _turn_2 10) (< _turn_2 15))
                        (for _ (range 2)
                          (`KismetArrayLibrary.Array_Remove` _chancestodoaction_3 (`KismetArrayLibrary.Array_LastIndex` _chancestodoaction_3)))
                        (elif (>= (`/Game/Blueprints/Core/PC_CardGame.Turn` (`self.PlayerControllerRef`)) 15)
                          (for _ (range 4)
                            (`KismetArrayLibrary.Array_Remove` _chancestodoaction_2 (`KismetArrayLibrary.Array_LastIndex` _chancestodoaction_2))))))
                    (:`then_1`
                      (`KismetArrayLibrary.Array_Shuffle` _chancestodoaction_4)
                      (if (`KismetArrayLibrary.Array_Random` _chancestodoaction_4)
                        (`self.HeavyAttack`)
                        (`self.StartMinionsSequence`)
                        (return)
                        (else
                          (`self.BaseAttack` :!label _label_2)
                          (`self.StartMinionsSequence`)
                          (return)))))
                  (else
                    (goto _label_2)))))))
        (else
          (goto _label))))
    (else
      (`self.BossMadnessAction`))))

(fn `BossMadnessAction`
  (locals (MadnessIndexAction :type Integer))
  (bind _output_get (set `local.MadnessIndexAction` (`KismetMathLibrary.RandomIntegerInRange` 0 2)))
  (switch `int` _output_get
    (:`0`
      (`self.BaseAttack`))
    (:`1`
      (`self.HeavyAttack`))
    (:`2`
      (`self.SpawnMinions`))))

(fn `EnnemyDeath`
  (bind _bossref (`/Game/Blueprints/Core/PC_CardGame.BossRef` (`self.PlayerControllerRef`)))
  (if (`self.IsBoss`)
    (`/Game/Blueprints/Core/PC_CardGame.FinishGame` (`self.PlayerControllerRef`) true)
    (else
      (`self.SetHealth` _bossref (`self.DamageRemains`))
      (for _array_element (`/Game/Blueprints/Core/Ennemies/BP_Ennemy_Master.MinionsSlots` _bossref)
        (set `/Game/Blueprints/Core/Cards/BP_CardSlot.IsEmpty` (== (`/Game/Blueprints/Core/Cards/BP_CardSlot.MinionRef` _array_element) self) _array_element))
      (`self.K2_DestroyActor`))))

(fn `InflictStatus`
  (params (PlayerRef :type "/Game/Blueprints/Core/Cards/BP_Card_Character Object Reference") (MinionRef :type "/Game/Blueprints/Core/Ennemies/BP_Ennemy_Master Object Reference"))
  (bind _playerref (`local.PlayerRef`))
  (bind _minionref (`local.MinionRef`))
  (if (`|EnumInequality` (`self.StatusToInflict`) "NewEnumerator6")
    (`/Engine/EditorBlueprintResources/StandardMacros.IsValid` PlayerRef
      (:`Is Valid`
        (if (`|EnumEquality` (`/Game/Blueprints/Core/Cards/BP_Card_Character.Status` (`local.PlayerRef`)) "NewEnumerator6")
          (if (== (`KismetMathLibrary.RandomIntegerInRange` 0 2) 0)
            (set `/Game/Blueprints/Core/Cards/BP_Card_Character.Status` (`self.StatusToInflict`) _playerref)
            (`/Game/Blueprints/Core/Cards/BP_Card_Character.VerifyStatus` _playerref))))
      (:`Is Not Valid`
        (if (`|EnumEquality` (`/Game/Blueprints/Core/Ennemies/BP_Ennemy_Master.Status` (`local.MinionRef`)) "NewEnumerator6")
          (if (== (`KismetMathLibrary.RandomIntegerInRange` 0 2) 0)
            (set `/Game/Blueprints/Core/Ennemies/BP_Ennemy_Master.Status` (`self.StatusToInflict`) _minionref)
            (`self.VerifyStatus` _minionref)))))))

(fn `SetHealth`
  (params (Value :type Integer))
  (bind _returnvalue (+ (`self.HP`) Value))
  (if (<= _returnvalue 0)
    (set `self.DamageRemains` _returnvalue)
    (set `self.HP` 0)
    (`self.EnnemyDeath`)
    (elif (> _returnvalue (`self.MaxHP`))
      (set `self.HP` (`self.MaxHP`))
      (else
        (set `self.HP` (+ (`self.HP`) (`local.Value`)))))))

(fn `UserConstructionScript`)

(fn `VerifyStatus`
  (returns (CanAct :type Boolean))
  (locals (TempStatus :type "/Game/Blueprints/Datas/Cards/Characters/E_Debuffs Enum") (TurnPassedWithStatus :type Integer) (BlindedCanAct :type "Array of Boolean") (StatusHealItself :type Boolean))
  (bind _blindedcanact (`local.BlindedCanAct`))
  (bind _turnpassedwithstatus (`local.TurnPassedWithStatus`))
  (if (`|EnumInequality` (`self.Status`) "NewEnumerator6")
    (if (`|EnumInequality` (`local.TempStatus`) (`self.Status`))
      (set `local.TempStatus` (`self.Status`))
      (set `local.TurnPassedWithStatus` 0)
      (else
        (`/Engine/EditorBlueprintResources/StandardMacros.IncrementInt` (`local.TurnPassedWithStatus`)
          (:`  `
            (switch `/Game/Blueprints/Datas/Cards/Characters/E_Debuffs` (`self.Status`)
              (:`NewEnumerator0`
                (if (< (`local.TurnPassedWithStatus`) 5)
                  (bind _output_get (set `local.StatusHealItself` (`KismetMathLibrary.RandomBool`)))
                  (if _output_get
                    (set `self.Status` "NewEnumerator6")
                    (return true)
                    (else
                      (return false)))
                  (else
                    (set `self.Status` "NewEnumerator6")
                    (return true))))
              (:`NewEnumerator1`
                (return (`KismetMathLibrary.RandomBool`)))
              (:`NewEnumerator2`
                (`KismetArrayLibrary.Array_Shuffle` _blindedcanact)
                (return (`KismetArrayLibrary.Array_Random` _blindedcanact)))
              (:`NewEnumerator3`
                (`self.SetHealth` (`KismetMathLibrary.FTrunc` (* (`self.MaxHP`) -0.1))))
              (:`NewEnumerator4`
                (return false))
              (:`NewEnumerator5`
                _)
              (:`NewEnumerator7`
                (return true))
              (:`NewEnumerator8`
                (return true))
              (:`NewEnumerator9`
                (return true))
              (:`NewEnumerator10`
                (return true)))
            (if (and (> _turnpassedwithstatus 2) (< _turnpassedwithstatus 5))
              (bind _output_get_2 (set `local.StatusHealItself` (`KismetMathLibrary.RandomBool`)))
              (if _output_get_2
                (set `self.Status` "NewEnumerator6")
                (return true)
                (else
                  (return true)))
              (elif (== (`local.TurnPassedWithStatus`) 5)
                (set `self.Status` "NewEnumerator6")
                (return true)
                (else
                  (return true))))))))
    (else
      (return true))))