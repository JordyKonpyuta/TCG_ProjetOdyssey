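; BP_Card_Tarot is a child card Blueprint for a clickable tarot card in the card game.
; On BeginPlay it binds and fires card initialisation, writing the tarot name into a WBP_Card_Character widget, and caches the PC_CardGame controller.
; Hovering shows or hides the description in the tarot UI.
; Clicking removes that UI and either starts the controller's selection mode or uses the card directly, depending on its target type.
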(event `self.ReceiveBeginPlay`
  (`parent.ReceiveBeginPlay`)
  (add `self.InitCard` (delegate `InitializeCard`))
  (`self.InitCard`)
  (bind _aspc_card_game (cast `/Game/Blueprints/Core/PC_CardGame` (`GameplayStatics.GetPlayerController` 0)))
  (set `self.PlayerControllerRef` _aspc_card_game))

(event `InitializeCard`
  (bind _aswbp_card_character (cast `/Game/Blueprints/Widgets/InGame/WBP_Card_Character` (`WidgetComponent.GetWidget` (`self.Widget_Card`))))
  (`TextBlock.SetText` (`/Game/Blueprints/Widgets/InGame/WBP_Card_Character.Text_Name` _aswbp_card_character) (`/Game/Blueprints/Datas/Cards/PDA_CardStats.Name` (`self.TarotData`))))

(event `self.Widget_Card.OnBeginCursorOver`
  (params (TouchedComponent :type "PrimitiveComponent Object Reference"))
  (`/Game/Blueprints/Widgets/InGame/WBP_TarotSpawn.SetDescriptionText` (`self.UI_TarotRef`) (`self.TarotData`)))

(event `self.Widget_Card.OnEndCursorOver`
  (params (TouchedComponent :type "PrimitiveComponent Object Reference"))
  (`/Game/Blueprints/Widgets/InGame/WBP_TarotSpawn.HideDescriptionText` (`self.UI_TarotRef`)))

(event `self.Widget_Card.OnClicked`
  (params (TouchedComponent :type "PrimitiveComponent Object Reference") (ButtonPressed :type "Key Structure"))
  (if (`|EnumEquality` (`/Game/Blueprints/Datas/Cards/Tarot/PDA_CardStats_Tarot.Target` (`self.TarotData`)) "NewEnumerator3")
    (`/Game/Blueprints/Core/PC_CardGame.SelectionMode` :`self` (`self.PlayerControllerRef`) :`TarotCard` self)
    (`Widget.RemoveFromParent` (`self.UI_TarotRef`))
    (else
      (`/Game/Blueprints/Core/PC_CardGame.UseTarotCard` (`self.PlayerControllerRef`) self)
      (`Widget.RemoveFromParent` (`self.UI_TarotRef`)))))

(fn `UserConstructionScript`
  (`parent.UserConstructionScript`))