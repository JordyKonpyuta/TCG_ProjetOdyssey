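; Stylized Death actor for the card game that appears over a killed card and performs an attack animation.
; It registers itself as DeathRef on PC_CardGame at BeginPlay.
; KillCard unhides it, moves it to the given card transform and plays AM_Attack.
; The montage's notify end hides the actor and calls CallDiscardCard, tying the discard to the animation's timing.
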(event `self.ReceiveBeginPlay`
  (set `/Game/Blueprints/Core/PC_CardGame.DeathRef` self (cast `/Game/Blueprints/Core/PC_CardGame` (`GameplayStatics.GetPlayerController` 0) :!pure true)))

(event `KillCard`
  (params (CardPosition :type "Transform Structure"))
  (`self.SetActorHiddenInGame` false)
  (`self.K2_SetActorTransform` CardPosition)
  (`|PlayMontage` (`self.SkeletalMesh`) "/Game/Assets/Stylized_Death/Meshes/Animation/AM_Attack.AM_Attack"
    (:`OnNotifyEnd`
      (`self.SetActorHiddenInGame` true)
      (`self.DiscardCard`))))

(fn `UserConstructionScript`)