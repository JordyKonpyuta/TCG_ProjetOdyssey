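; Card actor for a card game that handles hover lift, travel into the hand or a pile, and cursor dragging for placement.
; Looping timers interpolate the mesh or actor toward targets, with hand positions derived from the camera spring arm and hand index.
; While dragging, the card follows the cursor hit and traces downward for a slot or character card, then calls placement validation.
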(event `self.ReceiveBeginPlay`
  ; Event Begin Play
  (set `self.ControllerRef` (cast `/Game/Blueprints/Core/PC_CardGame` (`GameplayStatics.GetPlayerController` 0) :!pure true))
  (`self.InitCard`))

(event `self.Widget_Card.OnBeginCursorOver`
  (params (TouchedComponent :type "PrimitiveComponent Object Reference"))
  ; Hover and Unhover card - rise a little the card
  (if (not (`self.IsPlaced`))
    (set `self.Destination` (`KismetMathLibrary.Conv_VectorToTransform` (`SceneComponent.RelativeLocation` (`self.Arrow_Destination`))))
    (bind _returnvalue (`KismetSystemLibrary.K2_SetTimerDelegate` (`|CreateDelegate` :!event `MoveCard`) 0.01 true))
    (set `self.RiseCardTimerHandle` _returnvalue)
    (elif (`self.IsFollowingCursor`)
      (`self.K2_SetActorRelativeLocation` (`SceneComponent.RelativeLocation` (`self.Arrow_Start`))))))

(event `self.Widget_Card.OnEndCursorOver`
  (params (TouchedComponent :type "PrimitiveComponent Object Reference"))
  ; Hover and Unhover card - rise a little the card
  (if (not (`self.IsPlaced`))
    (set `self.Destination` (`KismetMathLibrary.Conv_VectorToTransform` (`SceneComponent.RelativeLocation` (`self.Arrow_Start`))))
    (bind _returnvalue (`KismetSystemLibrary.K2_SetTimerDelegate` (`|CreateDelegate` :!event `MoveCard`) 0.01 true))
    (set `self.RiseCardTimerHandle` _returnvalue)
    (elif (`self.IsFollowingCursor`)
      (`self.K2_SetActorRelativeLocation` (`SceneComponent.RelativeLocation` (`self.Arrow_Start`))))))

(event `CardMovement`
  (params (Destination :type "Transform Structure"))
  ; Move Selected Card
  (set `self.Destination` Destination)
  (bind _returnvalue (`KismetSystemLibrary.K2_SetTimerDelegate` (delegate `SelectCard`) 0.01 true))
  (set `self.RiseCardTimerHandle` _returnvalue))

(event `SelectCard`
  (bind _returnvalue (`self.GetTransform`))
  ; Move Selected Card
  (`self.K2_SetActorTransform` (`KismetMathLibrary.TInterpTo` _returnvalue (`self.Destination`) (`GameplayStatics.GetWorldDeltaSeconds`) 15.0))
  (if (`KismetMathLibrary.NearlyEqual_TransformTransform` _returnvalue (`self.Destination`) 0.5 0.5 0.5)
    (`KismetSystemLibrary.K2_ClearAndInvalidateTimerHandle` (`self.RiseCardTimerHandle`))))

(event `MoveCard`
  (bind _destination_location (`KismetMathLibrary.BreakTransform` (`self.Destination`)))
  (bind _destination_location_2 (`KismetMathLibrary.BreakTransform` (`self.Destination`)))
  (bind _staticmesh (`self.StaticMesh`))
  ; Function to call when Hover/Unhover card
  (`SceneComponent.K2_SetRelativeLocation` _staticmesh (`KismetMathLibrary.VInterpTo` (`SceneComponent.RelativeLocation` _staticmesh) _destination_location_2 (`GameplayStatics.GetWorldDeltaSeconds`) 3.0) false false)
  (if (== (`SceneComponent.RelativeLocation` _staticmesh) _destination_location :`ErrorTolerance` 50.0)
    (`KismetSystemLibrary.K2_ClearAndInvalidateTimerHandle` (`self.RiseCardTimerHandle`))))

(event `MoveToPile`
  (params (PileToMove :type "/Game/Blueprints/Core/Cards/BP_CardSlot Object Reference"))
  ; Move To Pile
  (`self.K2_SetActorLocation` (`KismetMathLibrary.VInterpTo` (`self.K2_GetActorLocation`) (`self.K2_GetActorLocation` PileToMove) (`GameplayStatics.GetWorldDeltaSeconds`) 30.0))
  (`/Game/Blueprints/Core/Cards/BP_CardSlot.AddCardOnPile` PileToMove self)
  (set `self.CanBeSelected` false)
  (`self.RemovePlayerCardFromSlots`))

(event `HandMovement`
  ; Place Card on Hand from Deck
  (bind _returnvalue (`KismetSystemLibrary.K2_SetTimerDelegate` (delegate `MoveInHand`) 0.01 true))
  (set `self.PlaceCardTimerHandle` _returnvalue))

(event `MoveInHand`
  (bind _returnvalue (`self.GetTransform`))
  (bind _returnvalue_2 (`self.GetTransform`))
  (bind _returnvalue_3 (`self.GetTransform`))
  (bind _controllerref (`self.ControllerRef`))
  (bind _returnvalue_location (`KismetMathLibrary.BreakTransform` (`SceneComponent.GetSocketTransform` (`/Game/Blueprints/Core/BP_CameraPlayer.SpringArm` (`/Game/Blueprints/Core/PC_CardGame.CameraRef` _controllerref)) "None" "RTS_World")))
  (bind _returnvalue_4 (`SceneComponent.GetSocketTransform` (`/Game/Blueprints/Core/BP_CameraPlayer.SpringArm` (`/Game/Blueprints/Core/PC_CardGame.CameraRef` (`self.ControllerRef`))) "None" "RTS_World"))
  (bind _returnvalue_5 (`SceneComponent.GetSocketTransform` (`/Game/Blueprints/Core/BP_CameraPlayer.SpringArm` (`/Game/Blueprints/Core/PC_CardGame.CameraRef` (`self.ControllerRef`))) "None" "RTS_World"))
  (bind _returnvalue_6 (`KismetMathLibrary.MakeTransform` (- _returnvalue_location (1000.0 0.0 1500.0)) (struct :`Yaw` -90.0 :`Roll` 40.0)))
  (bind _returnvalue_7 (`KismetMathLibrary.MakeTransform` (`KismetMathLibrary.MakeVector` (- (.x (.location _returnvalue_4)) 1000.0) (.y (.location _returnvalue_4)) (+ (- (.z (.location _returnvalue_4)) 1500.0) (* 20 (`KismetArrayLibrary.Array_Find` (`/Game/Blueprints/Core/PC_CardGame.Hand` (`self.ControllerRef`)) self)))) (struct :`Yaw` -90.0 :`Roll` 40.0)))
  ; Place Card on Hand from Deck
  (if (`KismetArrayLibrary.Array_IsEmpty` (`/Game/Blueprints/Core/PC_CardGame.Hand` _controllerref))
    (`self.K2_SetActorTransform` (`KismetMathLibrary.TInterpTo` _returnvalue_3 _returnvalue_6 (`GameplayStatics.GetWorldDeltaSeconds`) 15.0))
    (if (`KismetMathLibrary.NearlyEqual_TransformTransform` _returnvalue_3 _returnvalue_6 5.0 5.0)
      (`KismetSystemLibrary.K2_ClearAndInvalidateTimerHandle` (`self.PlaceCardTimerHandle`))
      (set `self.IsPlaced` false))
    (else
      (for _index (range (+ (`KismetArrayLibrary.Array_Find` (`/Game/Blueprints/Core/PC_CardGame.Hand` (`self.ControllerRef`)) self) 1))
        (bind _returnvalue_8 (`KismetMathLibrary.TInterpTo` _returnvalue (`KismetMathLibrary.MakeTransform` (`KismetMathLibrary.MakeVector` (- (.x (.location _returnvalue_5)) 1000.0) (- (.y (.location _returnvalue_5)) (* _index 200)) (+ (- (.z (.location _returnvalue_5)) 1500.0) (* _index 20))) (struct :`Yaw` -90.0 :`Roll` 40.0)) (`GameplayStatics.GetWorldDeltaSeconds`) 15.0))
        (`self.K2_SetActorTransform` _returnvalue_8)
        (if (`KismetMathLibrary.NearlyEqual_TransformTransform` _returnvalue _returnvalue_8 50.0 50.0)
          (`KismetSystemLibrary.K2_ClearAndInvalidateTimerHandle` (`self.PlaceCardTimerHandle`))
          (set `self.IsPlaced` false)))
      (`KismetSystemLibrary.K2_UnPauseTimerHandle` (`self.PlaceCardTimerHandle`))
      (`self.K2_SetActorTransform` (`KismetMathLibrary.TInterpTo` _returnvalue_2 _returnvalue_7 (`GameplayStatics.GetWorldDeltaSeconds`) 15.0))
      (if (`KismetMathLibrary.NearlyEqual_TransformTransform` _returnvalue_2 _returnvalue_7 5.0 5.0)
        (`KismetSystemLibrary.K2_ClearAndInvalidateTimerHandle` (`self.PlaceCardTimerHandle`))
        (set `self.IsPlaced` false)))))

(fn `SetCardToMousePosition`
  (locals (OtherCardsOnBoard :type "Array of /Game/Blueprints/Core/Cards/BP_Card Object Reference"))
  (bind _returnvalue (`self.K2_GetActorLocation`))
  (set `self.IsFollowingCursor` true)
  (`self.K2_SetActorLocation` (`KismetMathLibrary.VInterpTo` (`self.K2_GetActorLocation`) (`.Location` (`GameplayStatics.BreakHitResult` (`PlayerController.GetHitResultUnderCursorForObjects` (`self.ControllerRef`) (`|MakeArray` "ObjectTypeQuery1" :!type "EObjectTypeQuery Enum") true))) (`GameplayStatics.GetWorldDeltaSeconds`) 15.0))
  (bind _outhit (`KismetSystemLibrary.LineTraceSingle` :`Start` (+ _returnvalue (0.0 0.0 200.0)) :`End` (- _returnvalue (0.0 0.0 500.0)) :`TraceChannel` "TraceTypeQuery1" :`DrawDebugType` "Persistent"))
  (bind (_bblockinghit _binitialoverlap _time _distance _location _impactpoint _normal _impactnormal _physmat _hitactor) (`GameplayStatics.BreakHitResult` _outhit))
  (bind _asbp_card_slot (cast `/Game/Blueprints/Core/Cards/BP_CardSlot` _hitactor)
    (:`then`
      (set `self.SlotToAttach` _asbp_card_slot)
      (`self.VerifyIfCanPlaceCard`))
    (:`CastFailed`
      (bind _asbp_card_character (cast `/Game/Blueprints/Core/Cards/BP_Card_Character` _hitactor)
        (:`then`
          (set `self.CardToAttach` _asbp_card_character)
          (`self.VerifyIfCanPlaceCard`))
        (:`CastFailed`
          (set `self.CardToAttach` null)
          (set `self.SlotToAttach` null)
          (set `self.CanBePlaced` false))))))

(fn `UserConstructionScript`)