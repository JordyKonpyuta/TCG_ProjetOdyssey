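; Equipment card Blueprint that lets a card be dropped onto another card in a slot to equip it.
; On BeginPlay it binds a placement check that accepts the hovered slot only if its card's equipment entry for that piece type (weapon, armor or accessory) is empty.
; On click, a valid placement stores and applies the equipment, then moves this card to the Graveyard; otherwise it stops following the cursor and runs HandMovement.
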(event `OnClicked_Event`
  (params (TouchedActor :type "Actor Object Reference") (ButtonPressed :type "Key Structure" :default "None"))
  (bind _equipmentdata (`self.EquipmentData`))
  ; Click Event
  (if (`self.CanBePlaced`)
    (`KismetArrayLibrary.Array_Set` (`/Game/Blueprints/Core/Cards/BP_Card_Character.Equipment` (`/Game/Blueprints/Core/Cards/BP_CardSlot.CardAttached` (`self.SlotToAttach`))) (select `/Game/Blueprints/Datas/Cards/E_EquipmentType` (`/Game/Blueprints/Datas/Cards/PDA_CardStats_Equipment.Piece` _equipmentdata) :`NewEnumerator1` 1 :`NewEnumerator2` 2) _equipmentdata true)
    (`/Game/Blueprints/Core/Cards/BP_Card_Character.AddEquipment` (`/Game/Blueprints/Core/Cards/BP_CardSlot.CardAttached` (`self.SlotToAttach`)) _equipmentdata)
    (`self.MoveToPile` (`/Game/Blueprints/Core/PC_CardGame.Graveyard` (`self.ControllerRef`)))
    (else
      (set `self.IsFollowingCursor` false)
      (`KismetSystemLibrary.K2_ClearAndInvalidateTimerHandle` (`self.CursorTimerHandle`))
      (`self.HandMovement`))))

(event `self.ReceiveBeginPlay`
  ; Event Construct
  (`parent.ReceiveBeginPlay`)
  (add `self.VerifyIfCanPlaceCard` (delegate `VerifyIfCanPlaceEquipment`)))

(event `VerifyIfCanPlaceEquipment`
  ; Event Construct
  (if (== (`|GetArrayItem` (`/Game/Blueprints/Core/Cards/BP_Card_Character.Equipment` (`/Game/Blueprints/Core/Cards/BP_CardSlot.CardAttached` (`self.SlotHitted`))) (select `/Game/Blueprints/Datas/Cards/E_EquipmentType` (`/Game/Blueprints/Datas/Cards/PDA_CardStats_Equipment.Piece` (`self.EquipmentData`)) :`NewEnumerator1` 1 :`NewEnumerator2` 2)) null)
    (set `self.CanBePlaced` true)
    (set `self.SlotToAttach` (`self.SlotHitted`))
    (else
      (set `self.CanBePlaced` false)
      (set `self.SlotToAttach` null))))

(fn `UserConstructionScript`
  (`parent.UserConstructionScript`))