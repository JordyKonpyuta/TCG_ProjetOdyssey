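; BP_CardData holds a character card's runtime Attack, Defense and HP, pushing changes to the attached slot's card widget.
; Setters treat inputs as deltas, flooring at zero; HP also caps at CharacterData's value.
; SetHealth adds the slot's equipment modifier and applies defense debuffs.
; HP dropping below zero stores overflow damage on the slot and, if CanDie, triggers a matching equipment effect and the death animation.
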(fn `SetAttack`
  (params (NewValue :type Integer))
  (if (< (+ NewValue (`self.Attack`)) 0)
    (set `self.Attack` 0)
    (`/Game/Blueprints/Widgets/InGame/Cards/WBP_Card_Character.UpdateAttack` (cast `/Game/Blueprints/Widgets/InGame/Cards/WBP_Card_Character` (`WidgetComponent.GetWidget` (`/Game/Blueprints/Core/Cards/BP_CardSlot.Widget_Card` (`self.SlotAttached`))) :!pure true) 0)
    (else
      (bind _output_get (set `self.Attack` (+ (`self.Attack`) (`local.NewValue`))))
      (`/Game/Blueprints/Widgets/InGame/Cards/WBP_Card_Character.UpdateAttack` (cast `/Game/Blueprints/Widgets/InGame/Cards/WBP_Card_Character` (`WidgetComponent.GetWidget` (`/Game/Blueprints/Core/Cards/BP_CardSlot.Widget_Card` (`self.SlotAttached`))) :!pure true) _output_get))))

(fn `SetDefense`
  (params (NewValue :type Integer))
  (if (< (+ NewValue (`self.Defense`)) 0)
    (set `self.Defense` 0)
    (`/Game/Blueprints/Widgets/InGame/Cards/WBP_Card_Character.UpdateDefense` (cast `/Game/Blueprints/Widgets/InGame/Cards/WBP_Card_Character` (`WidgetComponent.GetWidget` (`/Game/Blueprints/Core/Cards/BP_CardSlot.Widget_Card` (`self.SlotAttached`))) :!pure true) 0)
    (else
      (bind _output_get (set `self.Defense` (+ (`self.Defense`) (`local.NewValue`))))
      (`/Game/Blueprints/Widgets/InGame/Cards/WBP_Card_Character.UpdateDefense` (cast `/Game/Blueprints/Widgets/InGame/Cards/WBP_Card_Character` (`WidgetComponent.GetWidget` (`/Game/Blueprints/Core/Cards/BP_CardSlot.Widget_Card` (`self.SlotAttached`))) :!pure true) _output_get))))

(fn `SetHealth`
  (params (NewValue :type Integer) (EnnemyToVerif :type "/Game/Blueprints/Core/Ennemies/BP_Ennemy_Master Object Reference") (AllyToVerif :type "/Game/Blueprints/Core/Cards/BP_CardData Object Reference"))
  (bind _hp (`/Game/Blueprints/Datas/Cards/Characters/PDA_CardStats_Character.HP` (`self.CharacterData`)))
  (bind _finaldamages (`/Game/Blueprints/Core/Cards/BP_CardSlot.EquipmentEffect` (`self.SlotAttached`) 1 NewValue EnnemyToVerif AllyToVerif))
  (bind _returnvalue (+ _finaldamages (`local.NewValue`)))
  (bind _returnvalue_2 (+ _returnvalue (`self.HP`)))
  (if (> _returnvalue_2 (`/Game/Blueprints/Datas/Cards/Characters/PDA_CardStats_Character.HP` (`self.CharacterData`)))
    (set `self.HP` _hp)
    (`/Game/Blueprints/Widgets/InGame/Cards/WBP_Card_Character.UpdateHealth` (cast `/Game/Blueprints/Widgets/InGame/Cards/WBP_Card_Character` (`WidgetComponent.GetWidget` (`/Game/Blueprints/Core/Cards/BP_CardSlot.Widget_Card` (`self.SlotAttached`))) :!pure true) _hp)
    (`/Game/Blueprints/Core/Cards/BP_CardSlot.ApplyDebuffOnDefense` (`self.SlotAttached`) (`local.AllyToVerif`) (`local.EnnemyToVerif`))
    (elif (< _returnvalue_2 0)
      (set `/Game/Blueprints/Core/Cards/BP_CardSlot.DamageRemains` _returnvalue_2 (`self.SlotAttached`))
      (set `self.HP` 0)
      (`/Game/Blueprints/Widgets/InGame/Cards/WBP_Card_Character.UpdateHealth` (cast `/Game/Blueprints/Widgets/InGame/Cards/WBP_Card_Character` (`WidgetComponent.GetWidget` (`/Game/Blueprints/Core/Cards/BP_CardSlot.Widget_Card` (`self.SlotAttached`))) :!pure true) 0)
      (`/Game/Blueprints/Core/Cards/BP_CardSlot.ApplyDebuffOnDefense` (`self.SlotAttached`) (`local.AllyToVerif`) (`local.EnnemyToVerif`))
      (if (`self.CanDie`)
        (for (_array_element _array_index) (`/Game/Blueprints/Core/Cards/BP_CardSlot.Equipment` (`self.SlotAttached`))
          (if (and (!= _array_element "/Game/Blueprints/Datas/Cards/Equipments/DA_Equipment_None.DA_Equipment_None") (`|EnumEquality` (`.Effect_18_AB09FEEA46604F3DCAC68F895421568B` (break `/Game/Blueprints/Datas/Cards/Equipments/S_EquipmentEffect` (`/Game/Blueprints/Datas/Cards/Equipments/PDA_CardStats_Equipment.Effect` _array_element))) "NewEnumerator2"))
            (`/Game/Blueprints/Core/Cards/BP_CardSlot.EquipmentEffect` (`self.SlotAttached`) _array_index 0 null null)
            (break)))
        (`KismetSystemLibrary.PrintString` null)
        (`/Game/Blueprints/Core/Cards/BP_CardSlot.DeathAnimation` (`self.SlotAttached`)))
      (else
        (bind _returnvalue_3 (+ (`self.HP`) _returnvalue))
        (set `self.HP` _returnvalue_3)
        (`/Game/Blueprints/Widgets/InGame/Cards/WBP_Card_Character.UpdateHealth` (cast `/Game/Blueprints/Widgets/InGame/Cards/WBP_Card_Character` (`WidgetComponent.GetWidget` (`/Game/Blueprints/Core/Cards/BP_CardSlot.Widget_Card` (`self.SlotAttached`))) :!pure true) _returnvalue_3)
        (`/Game/Blueprints/Core/Cards/BP_CardSlot.ApplyDebuffOnDefense` (`self.SlotAttached`) (`local.AllyToVerif`) (`local.EnnemyToVerif`))))))