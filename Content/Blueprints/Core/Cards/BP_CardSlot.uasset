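; Card slot actor for the card game, serving by type as deck, attack or defense slot, graveyard, discard pile or enemy target.
; On BeginPlay it registers player-side slots with PC_CardGame and shuffles the game instance's deck for the deck slot.
; Pile functions update the controller's card arrays and sacrifice/discard counts.
; In selection mode, clicking a targetable enemy slot toggles its minion in the attack's target list and refreshes the HUD.
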(event `self.ReceiveBeginPlay`
  ; Event Begin Play
  (set `self.PlayerControllerRef` (cast `/Game/Blueprints/Core/PC_CardGame` (`GameplayStatics.GetPlayerController` 0) :!pure true))
  (`self.InitSlot`))

(event `self.Plane.OnClicked`
  (params (TouchedComponent :type "PrimitiveComponent Object Reference") (ButtonPressed :type "Key Structure"))
  (bind _playercontrollerref (`self.PlayerControllerRef`))
  (bind _playercontrollerref_2 (`self.PlayerControllerRef`))
  (bind _playercontrollerref_3 (`self.PlayerControllerRef`))
  (bind _playercontrollerref_4 (`self.PlayerControllerRef`))
  (bind _selectedennemies (`/Game/Blueprints/Core/PC_CardGame.SelectedEnnemies` (`self.PlayerControllerRef`)))
  ; On Clicked (only to select ennemy on attack mode)
  (if (`/Game/Blueprints/Core/PC_CardGame.IsSelectionMode` (`self.PlayerControllerRef`))
    (if (and (`|EnumEquality` (`self.SlotType`) "NewEnumerator1") (`self.CanBeTargeted`))
      (`KismetSystemLibrary.PrintString` "Hello" true true (struct :`R` 1.0 :`G` 0.336281 :`A` 1.0))
      (if (`KismetArrayLibrary.Array_Contains` (`/Game/Blueprints/Core/PC_CardGame.SelectedEnnemies` _playercontrollerref_3) (`self.MinionRef`))
        (`KismetArrayLibrary.Array_RemoveItem` (`/Game/Blueprints/Core/PC_CardGame.SelectedEnnemies` (`self.PlayerControllerRef`)) (`self.MinionRef`))
        (bind _result (`/Engine/EditorBlueprintResources/StandardMacros.DecrementInt` (`/Game/Blueprints/Core/PC_CardGame.NumberOfCardsSelected` _playercontrollerref_4))
          (:`  `
            (`/Game/Blueprints/Widgets/InGame/WBP_HUD.ToggleSelectionMode` (`/Game/Blueprints/Core/PC_CardGame.HUD_Ref` _playercontrollerref_4) true (`/Game/Blueprints/Core/PC_CardGame.AttackToUse` _playercontrollerref_4) _result null)))
        (elif (< (`.NumberOfTargets_28_48B0234F465B0320CAA651B7085942FE` (break `/Game/Blueprints/Datas/Cards/Characters/S_CardAttacks` (`/Game/Blueprints/Core/PC_CardGame.AttackToUse` _playercontrollerref_3))) (`/Game/Blueprints/Core/PC_CardGame.NumberOfCardsSelected` (`self.PlayerControllerRef`)))
          (`KismetArrayLibrary.Array_Remove` _selectedennemies (`KismetArrayLibrary.Array_LastIndex` _selectedennemies))
          (`KismetArrayLibrary.Array_AddUnique` _selectedennemies (`self.MinionRef`))
          (bind _result_2 (`/Engine/EditorBlueprintResources/StandardMacros.IncrementInt` (`/Game/Blueprints/Core/PC_CardGame.NumberOfCardsSelected` _playercontrollerref_2))
            (:`  `
              (`/Game/Blueprints/Widgets/InGame/WBP_HUD.ToggleSelectionMode` (`/Game/Blueprints/Core/PC_CardGame.HUD_Ref` _playercontrollerref_2) true (`/Game/Blueprints/Core/PC_CardGame.AttackToUse` _playercontrollerref_2) _result_2 null)))
          (else
            (`KismetArrayLibrary.Array_AddUnique` _selectedennemies (`self.MinionRef`))
            (bind _result_3 (`/Engine/EditorBlueprintResources/StandardMacros.IncrementInt` (`/Game/Blueprints/Core/PC_CardGame.NumberOfCardsSelected` _playercontrollerref))
              (:`  `
                (`/Game/Blueprints/Widgets/InGame/WBP_HUD.ToggleSelectionMode` (`/Game/Blueprints/Core/PC_CardGame.HUD_Ref` _playercontrollerref) true (`/Game/Blueprints/Core/PC_CardGame.AttackToUse` _playercontrollerref) _result_3 null)))))))))

(fn `AddCardOnPile`
  (params (CardToAdd :type "/Game/Blueprints/Core/Cards/BP_CardData Object Reference"))
  (bind _cardtoadd (`local.CardToAdd`))
  (bind _playercontrollerref (`self.PlayerControllerRef`))
  (bind _cardtoadd_2 (`local.CardToAdd`))
  (bind _playercontrollerref_2 (`self.PlayerControllerRef`))
  (`|ExecutionSequence`
    (:`then_1`
      (`KismetArrayLibrary.Array_Add` (`self.CardsOnPile`) (`local.CardToAdd`))
      (if (`|EnumEquality` (`self.SlotType`) "NewEnumerator2")
        (set `/Game/Blueprints/Core/PC_CardGame.NumberOfSacrificiedCards` (+ (`/Game/Blueprints/Core/PC_CardGame.NumberOfSacrificiedCards` _playercontrollerref) 1) _playercontrollerref)
        (`/Game/Blueprints/Core/PC_CardGame.RemoveCardFromController` (`self.PlayerControllerRef`) (`local.CardToAdd`))
        (elif (`|EnumEquality` (`self.SlotType`) "NewEnumerator3")
          (set `/Game/Blueprints/Core/PC_CardGame.NumberOfDiscardedCards` (+ (`/Game/Blueprints/Core/PC_CardGame.NumberOfDiscardedCards` _playercontrollerref_2) 1) _playercontrollerref_2)
          (`/Game/Blueprints/Core/PC_CardGame.RemoveCardFromController` (`self.PlayerControllerRef`) (`local.CardToAdd`))
          (elif (`|EnumEquality` (`self.SlotType`) "NewEnumerator0")
            (`KismetArrayLibrary.Array_Set` (`/Game/Blueprints/Core/PC_CardGame.PlayerAttackCards` (`self.PlayerControllerRef`)) (`self.SlotIndex`) _cardtoadd_2 true)
            (set `self.CardAttached` _cardtoadd_2)
            (elif (`|EnumEquality` (`self.SlotType`) "NewEnumerator5")
              (`KismetArrayLibrary.Array_Set` (`/Game/Blueprints/Core/PC_CardGame.PlayerDefenseCards` (`self.PlayerControllerRef`)) (`self.SlotIndex`) _cardtoadd true)
              (set `self.CardAttached` _cardtoadd))))))))

(fn `InitSlot`
  (locals (CardToAdd :type "/Game/Blueprints/Datas/Cards/PDA_CardStats Object Reference") (SpawnPosition :type "Transform Structure"))
  (bind _slottype (`self.SlotType`))
  (bind _deck (`/Game/Blueprints/Core/GI_CardGameInstance.Deck` (cast `/Game/Blueprints/Core/GI_CardGameInstance` (`GameplayStatics.GetGameInstance`) :!pure true)))
  (if (`|EnumEquality` _slottype "NewEnumerator4")
    (`KismetArrayLibrary.Array_Shuffle` _deck)
    (for _array_element _deck
      (set `local.CardToAdd` _array_element))
    (set `/Game/Blueprints/Core/PC_CardGame.Deck` self (`self.PlayerControllerRef`))
    (elif (`|EnumEquality` _slottype "NewEnumerator0")
      (`KismetArrayLibrary.Array_Set` (`/Game/Blueprints/Core/PC_CardGame.PlayerAttackSlots` (`self.PlayerControllerRef`)) (`self.SlotIndex`) self)
      (elif (`|EnumEquality` _slottype "NewEnumerator5")
        (`KismetArrayLibrary.Array_Set` (`/Game/Blueprints/Core/PC_CardGame.PlayerDefenseSlots` (`self.PlayerControllerRef`)) (`self.SlotIndex`) self)
        (elif (`|EnumEquality` _slottype "NewEnumerator2")
          (set `/Game/Blueprints/Core/PC_CardGame.Graveyard` self (`self.PlayerControllerRef`))
          (elif (`|EnumEquality` _slottype "NewEnumerator3")
            (set `/Game/Blueprints/Core/PC_CardGame.DiscardPile` self (`self.PlayerControllerRef`))))))))

(fn `RemoveCardOnPile`
  (bind _playercontrollerref (`self.PlayerControllerRef`))
  (bind _playercontrollerref_2 (`self.PlayerControllerRef`))
  (if (`|EnumEquality` (`self.SlotType`) "NewEnumerator2")
    (set `/Game/Blueprints/Core/PC_CardGame.NumberOfSacrificiedCards` (- (`/Game/Blueprints/Core/PC_CardGame.NumberOfSacrificiedCards` _playercontrollerref) 1) _playercontrollerref)
    (elif (`|EnumEquality` (`self.SlotType`) "NewEnumerator3")
      (set `/Game/Blueprints/Core/PC_CardGame.NumberOfDiscardedCards` (- (`/Game/Blueprints/Core/PC_CardGame.NumberOfDiscardedCards` _playercontrollerref_2) 1) _playercontrollerref_2))))

(fn `ShuffleCards`
  (bind _cardsonpile (`self.CardsOnPile`))
  (`KismetArrayLibrary.Array_Shuffle` _cardsonpile)
  (for _ _cardsonpile
    _))

(fn `UserConstructionScript`)