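; BP_CardSlot is a card game slot that holds a pile of BP_Card actors.
; On BeginPlay, one slot type shuffles the GameInstance deck, then spawns and initializes a card per entry onto its pile.
; AddCardOnPile moves an existing card onto the pile and records it.
; Both paths place each card slightly above the top card, or the Arrow component if empty, rolled half a turn from that reference.
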(event `self.ReceiveBeginPlay`
  (bind _cardsonpile (`self.CardsOnPile`))
  (bind _returnvalue (`SceneComponent.K2_GetComponentToWorld` (`self.Arrow`)))
  (bind _deck (`/Game/Blueprints/Core/GI_CardGameInstance.Deck` (cast `/Game/Blueprints/Core/GI_CardGameInstance` (`GameplayStatics.GetGameInstance`) :!pure true)))
  (bind _returnvalue_2 (`self.GetTransform` (`|GetArrayItem` _cardsonpile (`KismetArrayLibrary.Array_LastIndex` _cardsonpile))))
  (if (`|EnumEquality` (`self.SlotType`) "NewEnumerator4")
    (`KismetArrayLibrary.Array_Shuffle` _deck)
    (for _array_element _deck
      (bind _returnvalue_3 (`|SpawnActorFromClass` "/Game/Blueprints/Core/BP_Card.BP_Card_C" (select `bool` (> (`KismetArrayLibrary.Array_Length` _cardsonpile) 0) :`false` (`KismetMathLibrary.MakeTransform` (+ (.location _returnvalue) (0.0 0.0 10.0)) (`KismetMathLibrary.MakeRotator` (+ (.roll (.rotation _returnvalue)) 180.0) (.pitch (.rotation _returnvalue)) (.yaw (.rotation _returnvalue))) (.scale _returnvalue)) :`true` (`KismetMathLibrary.MakeTransform` (+ (.location _returnvalue_2) (0.0 0.0 10.0)) (`KismetMathLibrary.MakeRotator` (+ (.roll (.rotation _returnvalue_2)) 180.0) (.pitch (.rotation _returnvalue_2)) (.yaw (.rotation _returnvalue_2))) (.scale _returnvalue_2)) :!type "Transform Structure") "Undefined" "MultiplyWithRoot" null null))
      (`/Game/Blueprints/Core/BP_Card.InitializeCard` _returnvalue_3 _array_element)
      (`KismetArrayLibrary.Array_Add` (`self.CardsOnPile`) _returnvalue_3))))

(fn `AddCardOnPile`
  (params (CardToAdd :type "/Game/Blueprints/Core/BP_Card Object Reference"))
  (bind _cardsonpile (`self.CardsOnPile`))
  (bind _returnvalue (`SceneComponent.K2_GetComponentToWorld` (`self.Arrow`)))
  (bind _returnvalue_2 (`self.GetTransform` (`|GetArrayItem` _cardsonpile (`KismetArrayLibrary.Array_LastIndex` _cardsonpile))))
  (`self.K2_SetActorTransform` CardToAdd (select `bool` (> (`KismetArrayLibrary.Array_Length` _cardsonpile) 0) :`false` (`KismetMathLibrary.MakeTransform` (+ (.location _returnvalue) (0.0 0.0 10.0)) (`KismetMathLibrary.MakeRotator` (+ (.roll (.rotation _returnvalue)) 180.0) (.pitch (.rotation _returnvalue)) (.yaw (.rotation _returnvalue))) (.scale _returnvalue)) :`true` (`KismetMathLibrary.MakeTransform` (+ (.location _returnvalue_2) (0.0 0.0 10.0)) (`KismetMathLibrary.MakeRotator` (+ (.roll (.rotation _returnvalue_2)) 180.0) (.pitch (.rotation _returnvalue_2)) (.yaw (.rotation _returnvalue_2))) (.scale _returnvalue_2)) :!type "Transform Structure") false false)
  (`KismetArrayLibrary.Array_Add` (`self.CardsOnPile`) CardToAdd))

(fn `UserConstructionScript`)