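; Player controller for the card game that creates and owns the UI for menu and gameplay levels.
; On BeginPlay it checks the level name, showing the main menu in LVL_Menu or the HUD elsewhere, with Game and UI input.
; Left mouse presses are forwarded to a widget interaction component as pointer clicks.
; SelectionMode resets the selected card count and switches the HUD into card selection for a chosen attack.
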(event `self.ReceiveBeginPlay`
  ; Event Begin Play
  (bind _returnvalue (`GameplayStatics.GetCurrentLevelName` true))
  (if (`KismetStringLibrary.NotEqual_StrStr` _returnvalue "LVL_Menu")
    (bind _returnvalue_2 (`|CreateWidget` "/Game/Blueprints/Widgets/InGame/WBP_HUD.WBP_HUD_C"))
    (bind _output_get (set `self.HUD_Ref` _returnvalue_2))
    (`UserWidget.AddToViewport` _output_get 0)
    (`WidgetBlueprintLibrary.SetInputMode_GameAndUIEx` self null "DoNotLock" true true)
    (`/Game/Blueprints/Widgets/InGame/WBP_HUD.ToggleSelectionMode` :`self` (`self.HUD_Ref`))
    (else
      (bind _returnvalue_3 (`|CreateWidget` "/Game/Blueprints/Widgets/Menu/WBP_MainMenu.WBP_MainMenu_C"))
      (`UserWidget.AddToViewport` _returnvalue_3 0)
      (`WidgetBlueprintLibrary.SetInputMode_GameAndUIEx` self _returnvalue_3 "DoNotLock" true true))))

(event `Key|LeftMouseButton`
  (params (Key :type "Key Structure"))
  (bind _widgetinteraction (`self.WidgetInteraction`))
  ; Attribute left mouse to widget interaction
  (:`Pressed`
    (`WidgetInteractionComponent.PressPointerKey` _widgetinteraction "LeftMouseButton"))
  (:`Released`
    (`WidgetInteractionComponent.ReleasePointerKey` _widgetinteraction "LeftMouseButton")))

(fn `SelectionMode`
  (params (AttackSelected :type "/Game/Blueprints/Datas/S_CardAttacks Structure"))
  (bind _output_get (set `self.IsSelectionMode` true))
  (bind _output_get_2 (set `self.NumberOfCardsSelected` 0))
  (`/Game/Blueprints/Widgets/InGame/WBP_HUD.ToggleSelectionMode` (`self.HUD_Ref`) _output_get AttackSelected _output_get_2))

(fn `UserConstructionScript`)